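; BP_WorstActor is an actor that runs deliberately wasteful math on overlap, apparently as a CPU load example.
; When a valid actor's capsule component begins overlapping its StaticMesh, it calls BadMathFunction CycleCount times in one synchronous loop.
; Each call combines Atan2 and Power of random floats into Calculation, which resets to zero after the loop, discarding the result.
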(event `self.StaticMesh.OnComponentBeginOverlap`
  (params (OverlappedComponent :type "PrimitiveComponent Object Reference") (OtherActor :type "Actor Object Reference") (OtherComp :type "PrimitiveComponent Object Reference") (OtherBodyIndex :type Integer) (bFromSweep :type Boolean) (SweepResult :type "HitResult Structure (by ref)"))
  (if (and (`KismetSystemLibrary.IsValid` OtherActor) (`.bSuccess` (cast `CapsuleComponent` OtherComp :!pure true)))
    (for _ (range 1 (+ (`self.CycleCount`) 1))
      (`self.BadMathFunction`))
    (set `self.Calculation` 0.0)))

(fn `BadMathFunction`
  (locals (LAtan2 :type "Float (double-precision)") (LPow :type "Float (double-precision)"))
  (set `local.LAtan2` (`KismetMathLibrary.Atan2` (`KismetMathLibrary.RandomFloatInRange` 0.0 1.0) (`KismetMathLibrary.RandomFloatInRange` 0.0 1.0)))
  (set `local.LPow` (`KismetMathLibrary.MultiplyMultiply_FloatFloat` (`KismetMathLibrary.RandomFloatInRange` 2.0 5.0) (`KismetMathLibrary.RandomFloatInRange` 2.0 5.0)))
  (set `self.Calculation` (+ (* (`local.LAtan2`) 2.0) (`local.LPow`))))

(fn `UserConstructionScript`)